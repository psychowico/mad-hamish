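; Player-controlled tank Blueprint that drives, aims and fires physics-driven shells.
; Axis inputs move and yaw the body, yaw the turret and roll the barrel through local transform offsets scaled by speed variables.
; FirePrimary spawns a Bullet at the Arrow and launches its cube with an impulse, using the particle system's active state to gate firing.
; Any Hit event destroys the tank's root component.
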(event `InputAction|FirePrimary`
  (params (Key :type "Key Structure"))
  (bind _arrow (`self.Arrow`))
  (bind _particlesystem (`self.ParticleSystem`))
  (bind _returnvalue (`SceneComponent.K2_GetComponentRotation` _arrow))
  (:`Pressed`
    (if (not (`ActorComponent.IsActive` _particlesystem))
      (`ActorComponent.Activate` _particlesystem false)
      (bind _returnvalue_2 (`|SpawnActorFromClass` "/Game/Blueprints/Bullet.Bullet_C" (`KismetMathLibrary.MakeTransform` (`SceneComponent.K2_GetComponentLocation` _arrow) _returnvalue) "AdjustIfPossibleButAlwaysSpawn" "OverrideRootScale" null null))
      (`PrimitiveComponent.AddImpulse` (`/Game/Blueprints/Bullet.Cube` _returnvalue_2) (* (`KismetMathLibrary.Conv_RotatorToVector` _returnvalue) 100000.0) "None" false))))

(event `InputAxis|Forward`
  (params (AxisValue :type "Float (single-precision)"))
  ;[1 1 1] Movement
  (`SceneComponent.K2_AddLocalOffset` (`self.tank_Body`) (`KismetMathLibrary.MakeVector` 0.0 (* AxisValue (`self.Speed`))) false false))

(event `InputAxis|Side`
  (params (AxisValue :type "Float (single-precision)"))
  ;[1 1 1] Movement
  (`SceneComponent.K2_AddLocalRotation` (`self.tank_Body`) (`KismetMathLibrary.MakeRotator` 0.0 0.0 (* AxisValue (`self.RotationSpeed`))) false false))

(event `InputAxis|LookLeft`
  (params (AxisValue :type "Float (single-precision)"))
  (`SceneComponent.K2_AddLocalRotation` (`self.tank_Turret`) (`KismetMathLibrary.MakeRotator` 0.0 0.0 (* AxisValue (`self.TurretSpeed`))) false false))

(event `self.ReceiveHit`
  (params (MyComp :type "PrimitiveComponent Object Reference") (Other :type "Actor Object Reference") (OtherComp :type "PrimitiveComponent Object Reference") (bSelfMoved :type Boolean) (HitLocation :type "Vector Structure") (HitNormal :type "Vector Structure") (NormalImpulse :type "Vector Structure") (Hit :type "HitResult Structure (by ref)"))
  (`ActorComponent.K2_DestroyComponent` (`self.RootComponent`)))

(event `InputAxis|LookUp`
  (params (AxisValue :type "Float (single-precision)"))
  (`SceneComponent.K2_AddLocalRotation` (`self.tank_Barrel`) (`KismetMathLibrary.MakeRotator` (* AxisValue (`self.BarrelSpeed`))) false false))

(fn `UserConstructionScript`)