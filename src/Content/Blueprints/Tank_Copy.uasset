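; Player-controlled tank Blueprint with a drivable body, rotating turret and elevating barrel, held to the surface beneath it by a custom downward pull.
; Axis inputs move and yaw the body scaled by delta time, while look inputs yaw the turret and roll the barrel within clamped limits, without delta-time scaling.
; Each tick, a trace along the body's local down finds the surface normal and applies a fixed impulse against it.
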(event `self.ReceiveTick`
  (params (DeltaSeconds :type "Float (single-precision)"))
  (bind _tank_body (`self.tank_Body`))
  (bind _returnvalue (`SceneComponent.K2_GetComponentLocation` _tank_body))
  (bind _outhit (`KismetSystemLibrary.LineTraceSingle` _returnvalue (- _returnvalue (`KismetMathLibrary.GreaterGreater_VectorRotator` (0.0 0.0 100000.0) (`SceneComponent.K2_GetComponentRotation` _tank_body))) "TraceTypeQuery1" true))
  (`PrimitiveComponent.AddImpulse` (`self.tank_Body`) (* (`.Normal` (`GameplayStatics.BreakHitResult` _outhit)) -100000.0) "None" false))

(event `InputAxis|Forward`
  (params (AxisValue :type "Float (single-precision)"))
  (`SceneComponent.K2_AddLocalOffset` (`self.tank_Body`) (`KismetMathLibrary.MakeVector` 0.0 (* (`GameplayStatics.GetWorldDeltaSeconds`) (* AxisValue (`self.Speed`)))) false false))

(event `InputAxis|Side`
  (params (AxisValue :type "Float (single-precision)"))
  (`SceneComponent.K2_AddLocalRotation` (`self.tank_Body`) (`KismetMathLibrary.MakeRotator` 0.0 0.0 (* (`GameplayStatics.GetWorldDeltaSeconds`) (* AxisValue (`self.RotationSpeed`)))) false false))

(event `InputAxis|LookLeft`
  (params (AxisValue :type "Float (single-precision)"))
  (`SceneComponent.K2_AddLocalRotation` (`self.tank_Turret`) (`KismetMathLibrary.MakeRotator` 0.0 0.0 (* AxisValue (`self.TurretSpeed`))) false false))

(event `InputAxis|LookUp`
  (params (AxisValue :type "Float (single-precision)"))
  (bind _tank_barrel (`self.tank_Barrel`))
  (bind (_relativerotation_roll _relativerotation_pitch _relativerotation_yaw) (`KismetMathLibrary.BreakRotator` (`SceneComponent.RelativeRotation` _tank_barrel)))
  (`SceneComponent.K2_AddLocalRotation` _tank_barrel (`KismetMathLibrary.MakeRotator` (* AxisValue (`self.BarrelSpeed`))) false false)
  (`SceneComponent.K2_SetRelativeRotation` _tank_barrel (`KismetMathLibrary.MakeRotator` (`KismetMathLibrary.ClampAngle` _relativerotation_roll -20.0 10.0) _relativerotation_pitch _relativerotation_yaw) false false))

(fn `UserConstructionScript`)